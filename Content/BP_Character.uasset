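; Character Blueprint that exercises file helper functions for listing, reading, creating and writing text files in a TestFolder directory.
; Every Tick, it scans the folder, reads each file and prints its name and content on screen with zero duration, giving a live view.
; Pressing K creates ThirdFile.txt in that folder and writes a fixed line of text to it.
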(event `self.ReceiveTick`
  (params (DeltaSeconds :type "Float (single-precision)"))
  (bind _files (`BPFileManager.FindFilesInDir` "TestFolder/"))
  (for _array_element _files
    (bind _savetexta (`BPFileManager.ReadText` (`KismetStringLibrary.Concat_StrStr` "TestFolder/" _array_element)))
    (`KismetSystemLibrary.PrintString` (`KismetStringLibrary.Concat_StrStr` "File: " _array_element "  |   Content: " _savetexta) true true (struct :`G` 0.66 :`B` 1.0 :`A` 1.0) 0.0)))

(event `Key|K` :consume false
  (params (Key :type "Key Structure"))
  (bind _returnvalue (`KismetStringLibrary.Concat_StrStr` "TestFolder/" "ThirdFile.txt"))
  (:`Pressed`
    (`BPFileManager.CreateFile` _returnvalue)
    (`BPFileManager.WriteText` "This is a general CPP library" _returnvalue)))

(fn `UserConstructionScript`)